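; Interactive keypad actor that the player views up close and clicks to enter a numeric code.
; E-Interact blends the view to the keypad, freezes movement and enables cursor clicks; Q restores normal control.
; Button clicks feed digits to Code, which updates the WBP_Keypad text and clears entry at five digits.
; A correct code notifies the player character, turns Spheres green and exits keypad view.
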(event OnClicked(button1)
  (params (TouchedComponent :type Primitive%20Component%20Object%20Reference) (ButtonPressed :type Key%20Structure))
  (CallFunction|Code "1"))

(event OnClicked(button2)
  (params (TouchedComponent :type Primitive%20Component%20Object%20Reference) (ButtonPressed :type Key%20Structure))
  (CallFunction|Code "2"))

(event OnClicked(button3)
  (params (TouchedComponent :type Primitive%20Component%20Object%20Reference) (ButtonPressed :type Key%20Structure))
  (CallFunction|Code "3"))

(event OnClicked(button4)
  (params (TouchedComponent :type Primitive%20Component%20Object%20Reference) (ButtonPressed :type Key%20Structure))
  (CallFunction|Code "4"))

(event OnClicked(button5)
  (params (TouchedComponent :type Primitive%20Component%20Object%20Reference) (ButtonPressed :type Key%20Structure))
  (CallFunction|Code "5"))

(event OnClicked(button6)
  (params (TouchedComponent :type Primitive%20Component%20Object%20Reference) (ButtonPressed :type Key%20Structure))
  (CallFunction|Code "6"))

(event OnClicked(button7)
  (params (TouchedComponent :type Primitive%20Component%20Object%20Reference) (ButtonPressed :type Key%20Structure))
  (CallFunction|Code "7"))

(event OnClicked(button8)
  (params (TouchedComponent :type Primitive%20Component%20Object%20Reference) (ButtonPressed :type Key%20Structure))
  (CallFunction|Code "8"))

(event OnClicked(button9)
  (params (TouchedComponent :type Primitive%20Component%20Object%20Reference) (ButtonPressed :type Key%20Structure))
  (CallFunction|Code "9"))

(event OnClicked(button0)
  (params (TouchedComponent :type Primitive%20Component%20Object%20Reference) (ButtonPressed :type Key%20Structure))
  (CallFunction|Code "0"))

(event EventBeginPlay
  (bind _aswbp_keypad (Utilities|Casting|CastToWBP_Keypad (UserInterface|GetWidget (Variables|Default|GetWidget))))
  (Variables|Default|SetAs%20WBP%20Keypad _aswbp_keypad))

(event EventE-Interact
  (bind _returnvalue (Game|GetPlayerController 0))
  (bind _returnvalue_2 (Game|GetPlayerController 0))
  (Game|Player|SetViewTargetwithBlend _returnvalue self 0.3 "VTBlend_Linear" 0.0 false)
  (Input|SetIgnoreLookInput _returnvalue false)
  (Variables|/Script/Engine.PlayerController|SetbEnableClickEvents _returnvalue true)
  (Variables|/Script/Engine.PlayerController|SetbShowMouseCursor _returnvalue true)
  (Pawn|Components|CharacterMovement|DisableMovement (Variables|/Script/Engine.Character|GetCharacterMovement (Game|GetPlayerCharacter 0)))
  (Input|EnableInput _returnvalue_2)
  (Input|SetInputModeGameandUI _returnvalue_2 0 "DoNotLock" true false))

(event Input|KeyboardEvents|Q
  (params (Key :type Key%20Structure))
  (:Pressed
    (|ExitKeypad)))

(fn ConstructionScript)

(fn Code
  (params (B :type String))
  (bind _returnvalue (Game|GetPlayerController 0))
  (bind _returnvalue_2 (Game|GetPlayerCharacter 0))
  (Audio|PlaySound2D "/Game/Keypad/Sounds/key_code_sfx.key_code_sfx" 1.0 1.0 0.0 0 0)
  (bind _output_get (Variables|Default|SetInput (Utilities|String|Append (Variables|Default|GetInput) B)))
  (Variables|Default|SetlengthOfCode (+ (Variables|Default|GetlengthOfCode) 1))
  (Rendering|Components|TextRender|SetText (Variables|/Game/Keypad/WBP_Keypad.WBP_Keypad_C|GetcodeText (Variables|Default|GetAs%20WBP%20Keypad)) (Utilities|Text|ToText(String) _output_get))
  (if (Utilities|Enum|Equal(Enum) (Variables|Default|GetInput) (Variables|Default|GetcorrectCode))
    (Class|BPIUnlockCodeDoor|SetCodeCorrect(Message) (Game|GetPlayerCharacter 0) true)
    (Rendering|Material|SetMaterial (Variables|Default|Getspheres) 0 "/Game/Keypad/MI_KGreen.MI_KGreen")
    (Input|DisableInput _returnvalue)
    (Game|Player|SetViewTargetwithBlend _returnvalue _returnvalue_2 0.3 "VTBlend_Linear" 0.0 false)
    (Input|ResetIgnoreLookInput _returnvalue)
    (Variables|/Script/Engine.PlayerController|SetbEnableClickEvents _returnvalue false)
    (Variables|/Script/Engine.PlayerController|SetbShowMouseCursor _returnvalue false)
    (Pawn|Components|CharacterMovement|SetMovementMode (Variables|/Script/Engine.Character|GetCharacterMovement _returnvalue_2) "MOVE_Walking" 0)
    (Input|SetInputModeGameOnly _returnvalue false))
  (if (>= (Variables|Default|GetlengthOfCode) 5)
    (bind _output_get_2 (Variables|Default|SetInput ""))
    (Rendering|Components|TextRender|SetText (Variables|/Game/Keypad/WBP_Keypad.WBP_Keypad_C|GetcodeText (Variables|Default|GetAs%20WBP%20Keypad)) (Utilities|Text|ToText(String) _output_get_2))
    (Variables|Default|SetlengthOfCode 0)))