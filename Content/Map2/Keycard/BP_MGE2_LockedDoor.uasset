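; A locked door on Map2 that opens only when the player character holds the MGE2 keycard.
; The E-Interact event reads the keycard flag on BP_FirstPersonCharacter, printing a locked message when it is false.
; With the keycard, a sound plays and a FlipFlop alternately plays or reverses a timeline that lerps the door's relative yaw, swinging it a quarter turn open or closed.
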(event EventBeginPlay)

(event Collision|EventActorBeginOverlap
  (params (OtherActor :type Actor%20Object%20Reference)))

(event EventTick
  (params (DeltaSeconds :type Float%20%28single-precision%29)))

(event EventE-Interact
  (bind _asbp_first_person_character (Utilities|Casting|CastToBP_FirstPersonCharacter (Game|GetPlayerCharacter 0)))
  (if (Variables|/Game/FirstPerson/Blueprints/BP_FirstPersonCharacter.BP_FirstPersonCharacter_C|GetHasMGE2Keycard _asbp_first_person_character)
    (Audio|PlaySound2D "/Game/SFX/Door_Opening_Sound_Effect.Door_Opening_Sound_Effect" 1.0 1.0 0.0 0 0)
    (Utilities|FlowControl|FlipFlop
      (:A
        (bind _doorfloat (Timeline|OpenDoor%20Timeline PlayFromStart)
          (:Update
            (Transformation|SetRelativeRotation (Variables|Default|GetDoor) (Math|Rotator|MakeRotator 0.0 0.0 (Math|Float|Lerp 0.0 -9e+01 _doorfloat)) false false))))
      (:B
        (Timeline|OpenDoor%20Timeline Reverse)))
    (else
      (Development|PrintString "\"Locked! Need Key.\""))))

(fn ConstructionScript)