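; BP_ExitDoor is the horror game's exit door, which ends the game when opened after all collectables are gathered.
; A sphere overlap enables E input for the first-person character, and pressing E checks CollectablesLeft on BP_HorrorGameMode.
; A FlipFlop plays or reverses a timeline that swings the door.
; The timeline's Update also runs a short Delay, then pauses the game and shows WBP_GameEnd with UI-only input.
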(event OnComponentBeginOverlap(Sphere)
  (params (OverlappedComponent :type Primitive%20Component%20Object%20Reference) (OtherActor :type Actor%20Object%20Reference) (OtherComp :type Primitive%20Component%20Object%20Reference) (OtherBodyIndex :type Integer) (bFromSweep :type Boolean) (SweepResult :type Hit%20Result%20Structure%20%28by%20ref%29))
  (Utilities|Casting|CastToBP_FirstPersonCharacter OtherActor)
  (Input|EnableInput (Game|GetPlayerController 0)))

(event OnComponentEndOverlap(Sphere)
  (params (OverlappedComponent :type Primitive%20Component%20Object%20Reference) (OtherActor :type Actor%20Object%20Reference) (OtherComp :type Primitive%20Component%20Object%20Reference) (OtherBodyIndex :type Integer))
  (Utilities|Casting|CastToBP_FirstPersonCharacter OtherActor)
  (Input|DisableInput (Game|GetPlayerController 0)))

(event Custom|OpenDoor)

(event EventBeginPlay)

(event Collision|EventActorBeginOverlap
  (params (OtherActor :type Actor%20Object%20Reference)))

(event EventTick
  (params (DeltaSeconds :type Float%20%28single-precision%29)))

(event Input|KeyboardEvents|E
  (params (Key :type Key%20Structure :default "None"))
  (:Pressed
    (bind _asbp_horror_game_mode (Utilities|Casting|CastToBP_HorrorGameMode (Game|GetGameMode)))
    (if (== (Variables|/Game/Variant_Horror/Blueprints/BP_HorrorGameMode.BP_HorrorGameMode_C|GetCollectablesLeft _asbp_horror_game_mode) 0)
      (Audio|PlaySound2D "/Game/SFX/Door_Opening_Sound_Effect.Door_Opening_Sound_Effect" 1.0 1.0 0.0 0 0)
      (Utilities|FlowControl|FlipFlop
        (:A
          (bind _doorfloat (Timeline|OpenDoor%20Timeline PlayFromStart)
            (:Update
              (Transformation|SetRelativeRotation (Variables|Default|GetDoor) (Math|Rotator|MakeRotator 0.0 0.0 (Math|Float|Lerp 0.0 -9e+01 _doorfloat)) false false)
              (Utilities|FlowControl|Delay 0.7)
              (Game|SetGamePaused true)
              (bind _returnvalue (UserInterface|CreateWidget "/Game/UI/WBP_GameEnd.WBP_GameEnd_C"))
              (UserInterface|Viewport|AddtoViewport _returnvalue 0)
              (Input|SetInputModeUIOnly (Game|GetPlayerController 0) _returnvalue "DoNotLock" false)
              (Variables|/Script/Engine.PlayerController|SetbShowMouseCursor (Game|GetPlayerController 0) true))))
        (:B
          (Timeline|OpenDoor%20Timeline Reverse))))))

(fn ConstructionScript)