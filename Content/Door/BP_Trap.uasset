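; BP_Trap is a moving trap actor that destroys the first-person player character on contact with its DamageBox.
; While ShouldDrop is true, Tick offsets it along local Z by DropVelocity each frame, without delta-time scaling; nothing here sets that flag.
; A Playsound event plays a quiet 2D chain cue.
; BeginPlay stores start and end locations, but the movement never reads them, so it has no stop point.
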(event OnComponentBeginOverlap(DamageBox)
  (params (OverlappedComponent :type Primitive%20Component%20Object%20Reference) (OtherActor :type Actor%20Object%20Reference) (OtherComp :type Primitive%20Component%20Object%20Reference) (OtherBodyIndex :type Integer) (bFromSweep :type Boolean) (SweepResult :type Hit%20Result%20Structure%20%28by%20ref%29))
  (bind _asbp_first_person_character (Utilities|Casting|CastToBP_FirstPersonCharacter OtherActor))
  (Actor|DestroyActor _asbp_first_person_character))

(event Custom|Playsound
  (Audio|PlaySound2D "/Game/Door/Sound/Chain_Cue.Chain_Cue" 0.2 1.0 0.0 0 0))

(event EventBeginPlay
  (Variables|Default|SetStartLocation (Transformation|GetActorLocation))
  (Variables|Default|SetEndLocation (- (Variables|Default|GetStartLocation) "0.000000,0.000000,-500.000000")))

(event Collision|EventActorBeginOverlap
  (params (OtherActor :type Actor%20Object%20Reference)))

(event EventTick
  (params (DeltaSeconds :type Float%20%28single-precision%29))
  (if (Variables|Default|GetShouldDrop)
    (Transformation|AddActorLocalOffset (Math|Vector|MakeVector 0.0 0.0 (Variables|Default|GetDropVelocity)) false false)))

(fn ConstructionScript)